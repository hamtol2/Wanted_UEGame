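; BP_Cube is a trigger cube that glows while overlapped and launches the player character along its arrow.
; On BeginPlay it creates a dynamic instance of M_Emissive on its mesh.
; Begin overlap prints the other actor's name and raises the emissive value; end overlap resets it to zero.
; Actors tagged Player that cast to BP_ThirdPersonCharacter receive a velocity-change impulse along the Arrow's forward vector, scaled by ImpulsePower.
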(event EventBeginPlay
  (bind _returnvalue (Rendering|Material|CreateDynamicMaterialInstance (Variables|Default|GetStaticMesh) 0 "/Game/Materials/M_Emissive.M_Emissive" "None" :!class /Script/Engine.PrimitiveComponent))
  (Variables|Default|SetMaterialInstance _returnvalue))

(event Collision|EventActorBeginOverlap
  (params (OtherActor :type Actor%20Object%20Reference))
  (Development|PrintString (Utilities|GetDisplayName OtherActor))
  (Rendering|Material|SetScalarParameterValue (Variables|Default|GetMaterialInstance) "Value" (Variables|효과|GetEmissivePower) :!class /Script/Engine.MaterialInstanceDynamic)
  (if (Actor|ActorHasTag OtherActor "Player")
    (bind _asbp_third_person_character (Utilities|Casting|CastToBP_ThirdPersonCharacter OtherActor))
    (Physics|AddImpulse (Variables|/Script/Engine.Character|GetCharacterMovement _asbp_third_person_character) (* (Math|Vector|GetForwardVector (Variables|Default|GetArrow)) (Variables|Default|GetImpulsePower)) true)))

(event EventTick
  (params (DeltaSeconds :type Float%20%28single-precision%29)))

(event Collision|EventActorEndOverlap
  (params (OtherActor :type Actor%20Object%20Reference))
  (Rendering|Material|SetScalarParameterValue (Variables|Default|GetMaterialInstance) "Value" 0.0 :!class /Script/Engine.MaterialInstanceDynamic))

(fn ConstructionScript)
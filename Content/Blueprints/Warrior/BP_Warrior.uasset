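; Player Warrior character with Enhanced Input movement, melee combat and health feedback.
; A State variable gates moving, jumping and attacking; attacks need a collected weapon and ground contact, play AM_Attack, and queue NextCombo from the current montage section.
; Attack events forward hit-check windows to the socketed weapon, add a forward dash and broadcast radial attacks.
; Damage feeds DamageReciver, updating the HP widget and material hit flash; death disables capsule collision and input mapping.
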(event Custom|OnAttackEnd
  ;[1 1 1] 공격 종료 처리
  (Variables|Default|SetState "NewEnumerator0"))

(event Custom|OnAttackCheckBegin
  ;[1 1 1] 공격 판정 시작/종료
  (Utilities|IsValid (Variables|Default|GetWeapon)
    (:Is%20Valid
      (Default|OnAttackCheckBegin (Variables|Default|GetWeapon)))))

(event Custom|OnAttackCheckEnd
  ;[1 1 1] 공격 판정 시작/종료
  (Utilities|IsValid (Variables|Default|GetWeapon)
    (:Is%20Valid
      (Default|OnAttackCheckEnd (Variables|Default|GetWeapon)))))

(event Custom|OnAttackDash
  ;[1 1 1] 공격 시 앞으로 슬라이드
  (Physics|AddImpulse (Variables|Character|GetCharacterMovement) (* (Transformation|GetActorForwardVector) (Variables|Default|GetDashPower)) true))

(event Custom|OnWeaponCollected
  (params (WeaponActor :type Actor%20Object%20Reference))
  (Actor|SetOwner WeaponActor self)
  (Transformation|AttachComponentToComponent WeaponActor (Variables|Character|GetMesh) "WeaponPosition" "SnapToTarget" "SnapToTarget" "SnapToTarget" true)
  (Variables|Default|SetbHasWeapon true)
  (bind _asbp_weapon (Utilities|Casting|CastToBP_Weapon WeaponActor))
  (Variables|Default|SetWeapon _asbp_weapon))

(event Custom|OnRadialAttack
  ;[1 1 1] Radial 이벤트 발행
  (Default|CallRadialAttackEvent))

(event Custom|OnDead
  (bind _returnvalue (Game|GetPlayerController 0))
  ;[1 1 1] 초기화
  ;;[1 1 1] 옵저버 패턴
  (Collision|SetCollisionEnabled (Variables|Collision|GetCapsuleComponent) "NoCollision")
  (Variables|Default|SetState "NewEnumerator2")
  (Utilities|IsValid _returnvalue
    (:Is%20Valid
      (Input|RemoveMappingContext (PlayerController|LocalPlayerSubsystems|GetEnhancedInputLocalPlayerSubsystem _returnvalue) "/Game/Blueprints/Inputs/IMC_Character.IMC_Character" "(bIgnoreAllPressedKeysUntilRelease=True,bForceImmediately=False,bNotifyUserSettings=False)"))))

(event Custom|OnHealthPowerChanged
  (Default|SetHPPercent (Variables|Default|GetHPHUD) (Default|GetHPPercent (Variables|Default|GetDamageReciver))))

(event Input|EnhancedActionEvents|EnhancedInputActionIA_Move
  (params (ActionValue :type Vector%202D%20Structure) (ElapsedSeconds :type Float%20%28double-precision%29) (TriggeredSeconds :type Float%20%28double-precision%29) (InputAction :type Input%20Action%20Object%20Reference :default "/Game/ThirdPerson/Input/Actions/IA_Move.IA_Move"))
  (bind _returnvalue (Pawn|GetControlRotation :!class /Script/Engine.Pawn))
  ;[0.6641 1 0.8335] 캐릭터 이동
  (switch Utilities|FlowControl|Switch|SwitchonE_WarriorState (Variables|Default|GetState)
    (:NewEnumerator0
      (Pawn|Input|AddMovementInput (+ (* (Math|Vector|GetForwardVector (Math|Rotator|MakeRotator 0.0 0.0 (.yaw _returnvalue))) (.y ActionValue)) (* (Math|Vector|GetRightVector (Math|Rotator|MakeRotator 0.0 0.0 (.yaw _returnvalue))) (.x ActionValue))) 1.0 false))))

(event Input|EnhancedActionEvents|EnhancedInputActionIA_Look
  (params (ActionValue :type Vector%202D%20Structure) (ElapsedSeconds :type Float%20%28double-precision%29) (TriggeredSeconds :type Float%20%28double-precision%29) (InputAction :type Input%20Action%20Object%20Reference :default "/Game/ThirdPerson/Input/Actions/IA_Look.IA_Look"))
  ;[1 1 1] 카메라 회전
  (Pawn|Input|AddControllerPitchInput (.y ActionValue))
  (Pawn|Input|AddControllerYawInput (.x ActionValue))
  (switch Utilities|FlowControl|Switch|SwitchonE_WarriorState (Variables|Default|GetState)
    (:NewEnumerator1
      (CallFunction|TurntoTarget))))

(event Input|EnhancedActionEvents|EnhancedInputActionIA_Attack
  (params (ActionValue :type Boolean) (ElapsedSeconds :type Float%20%28double-precision%29) (TriggeredSeconds :type Float%20%28double-precision%29) (InputAction :type Input%20Action%20Object%20Reference :default "/Game/Blueprints/Inputs/IA_Attack.IA_Attack"))
  ;[1 1 1] 공격 입력 처리
  (if (and (Variables|Default|GetbHasWeapon) (not (AI|Components|NavMovement|IsFalling (Variables|Character|GetCharacterMovement))))
    (if (Utilities|Enum|NotEqual(Enum) (Variables|Default|GetState) "NewEnumerator1")
      (Variables|Default|SetState "NewEnumerator1")
      (Animation|PlayAnimMontage "/Game/Blueprints/Warrior/AM_Attack.AM_Attack" 1.0 "Attack1")
      (else
        (switch name (Animation|Montage|MontageGetCurrentSection (Components|SkeletalMesh|GetAnimInstance (Variables|Character|GetMesh)) "/Game/Blueprints/Warrior/AM_Attack.AM_Attack")
          (:Attack1
            (Variables|Default|SetNextCombo "Attack2"))
          (:Attack2
            (Variables|Default|SetNextCombo "Attack3"))
          (:Attack3
            (Variables|Default|SetNextCombo "Attack4")))))))

(event Input|EnhancedActionEvents|EnhancedInputActionIA_Jump
  (params (ActionValue :type Boolean) (ElapsedSeconds :type Float%20%28double-precision%29) (TriggeredSeconds :type Float%20%28double-precision%29) (InputAction :type Input%20Action%20Object%20Reference :default "/Game/ThirdPerson/Input/Actions/IA_Jump.IA_Jump"))
  (switch Utilities|FlowControl|Switch|SwitchonE_WarriorState (Variables|Default|GetState)
    (:NewEnumerator0
      (Character|Jump))))

(event EventBeginPlay
  (bind _returnvalue (Game|GetPlayerController 0))
  ;[1 1 1] 초기화
  (Rendering|SetCastShadow (Variables|Default|GetHPBar) false)
  (Utilities|IsValid _returnvalue
    (:Is%20Valid
      (Input|AddMappingContext (PlayerController|LocalPlayerSubsystems|GetEnhancedInputLocalPlayerSubsystem _returnvalue) "/Game/Blueprints/Inputs/IMC_Character.IMC_Character" 0 "(bIgnoreAllPressedKeysUntilRelease=True,bForceImmediately=False,bNotifyUserSettings=False)")
      ;;[1 1 1] 옵저버 패턴
      (EventDispatchers|BindEventtoOnDead (Variables|Default|GetDamageReciver) (delegate Custom|OnDead))
      (bind _returnvalue_2 (Rendering|Material|CreateDynamicMaterialInstance (Variables|Character|GetMesh) 0 "/Game/InfinityBladeWarriors/Characters/TM/CharM_Warrior/M_Char_Warrior_Inst.M_Char_Warrior_Inst" "None" :!class /Script/Engine.PrimitiveComponent))
      (Variables|Default|SetDynamicInstance _returnvalue_2)
      (bind _aswbp_hphud (Utilities|Casting|CastToWBP_HPHUD (UserInterface|GetUserWidgetObject (Variables|Default|GetHPBar))))
      (Variables|Default|SetHPHUD _aswbp_hphud)
      (EventDispatchers|BindEventtoOnHealthPowerChanged (Variables|Default|GetDamageReciver) (delegate Custom|OnHealthPowerChanged)))))

(event Collision|EventActorBeginOverlap
  (params (OtherActor :type Actor%20Object%20Reference)))

(event EventTick
  (params (DeltaSeconds :type Float%20%28single-precision%29)))

(event Game|Damage|EventAnyDamage
  (params (Damage :type Float%20%28single-precision%29) (DamageType :type Damage%20Type%20Object%20Reference) (InstigatedBy :type Controller%20Object%20Reference) (DamageCauser :type Actor%20Object%20Reference))
  (bind _hphud (Variables|Default|GetHPHUD))
  (Default|ReceiveDamage (Variables|Default|GetDamageReciver) Damage)
  (Default|SetHPPercent _hphud (Default|GetHPPercent (Variables|Default|GetDamageReciver)))
  (Default|PlayTextAnimation _hphud (Math|Float|Truncate Damage))
  (bind _hitvalue (Timeline|DamageEffect PlayFromStart)
    (:Update
      (Rendering|Material|SetScalarParameterValue (Variables|Default|GetDynamicInstance) "HitValue" _hitvalue :!class /Script/Engine.MaterialInstanceDynamic))))

(fn ConstructionScript)

(fn TurntoTarget
  (Transformation|SetActorRotation (Math|Rotator|MakeRotfromX (Math|Vector|GetForwardVector (Math|Rotator|MakeRotator 0.0 0.0 (.yaw (Pawn|GetControlRotation :!class /Script/Engine.Pawn)))))))

(fn IsDead
  (return (Utilities|Enum|Equal(Enum) (Variables|Default|GetState) "NewEnumerator2")))
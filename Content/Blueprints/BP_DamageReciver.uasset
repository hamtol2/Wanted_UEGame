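; BP_DamageReciver is a Blueprint that tracks health for damage handling and signals death.
; HealthPower starts at MaxHealthPower on BeginPlay, and ReceiveDamage subtracts the incoming damage from it directly.
; When health drops to zero or below, it is clamped to zero and OnDead is called.
; There is no guard against repeat hits, so further damage at zero health can call OnDead again.
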(event Custom|ReceiveDamage
  (params (Damage :type Float%20%28double-precision%29))
  ;[1 1 1] 대미지 처리 공식
  (Variables|Default|SetHealthPower (- (Variables|Default|GetHealthPower) Damage))
  (if (<= (Variables|Default|GetHealthPower) 0.0)
    (Variables|Default|SetHealthPower 0.0)
    (Default|CallOnDead)))

(event EventBeginPlay
  (Variables|Default|SetHealthPower (Variables|Default|GetMaxHealthPower)))